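; BP_LoSPP is a line-of-sight post-process actor that pairs a PostProcess component with an orthographic scene capture covering the map.
; Its construction script centers the actor at world X/Y zero, keeping its height, and sets the capture's ortho width to MapDimension.
; The same MapDimension is written to the MPC_LoS parameter collection, so materials reading it share the capture's scale.
; BeginPlay enables the post process.
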(event EventBeginPlay
  (Variables|/Script/Engine.PostProcessComponent|SetbEnabled (Variables|Default|GetPostProcess) true))

(event Collision|EventActorBeginOverlap
  (params (OtherActor :type Actor%20Object%20Reference)))

(event EventTick
  (params (DeltaSeconds :type Float%20%28single-precision%29)))

(fn ConstructionScript
  (bind _scenecapturecomponent2d (Variables|Default|GetSceneCaptureComponent2D))
  (Transformation|SetActorLocation (Math|Vector|MakeVector 0.0 0.0 (.z (Transformation|GetActorLocation))) false false)
  (Rendering|Material|SetScalarParameterValue "/Game/Materials/MPC_LoS.MPC_LoS" "MapDimension" (Variables|Default|GetMapDimension) :!class /Script/Engine.KismetMaterialLibrary)
  (Variables|/Script/Engine.SceneCaptureComponent2D|SetProjectionType _scenecapturecomponent2d "Orthographic")
  (Variables|/Script/Engine.SceneCaptureComponent2D|SetOrthoWidth _scenecapturecomponent2d (Variables|Default|GetMapDimension)))